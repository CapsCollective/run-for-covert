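; Procedural terrain actor that builds a map from a random seed and a set of level positions, coordinated between server and clients.
; On BeginPlay the server picks the seed, stores the level positions and calls Generate.
; Clients call Generate when LevelPositions replicates, while the Seed RepNotify only prints the value.
; BPGenerate passes both replicated values to GenerateMap.
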(event `self.ReceiveBeginPlay`
  (if (`KismetSystemLibrary.IsServer`)
    (set `self.Seed` (`KismetMathLibrary.RandomIntegerInRange` -10000 10000))
    (bind _returnvalue (`self.GetLevelPositions`))
    (set `self.LevelPositions` _returnvalue)
    (`self.BP_Generate`)))

(fn `BP_Generate`
  (`self.GenerateMap` (`self.Seed`) (`self.LevelPositions`)))

(fn `OnRep_LevelPositions`
  (if (not (`KismetSystemLibrary.IsServer`))
    (`self.BP_Generate`)))

(fn `OnRep_Seed`
  (`KismetSystemLibrary.PrintString` (`KismetStringLibrary.Conv_IntToString` (`self.Seed`))))

(fn `UserConstructionScript`)