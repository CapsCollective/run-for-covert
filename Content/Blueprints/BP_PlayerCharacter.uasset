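; First-person player character Blueprint that adds cosmetic feedback for damage, firing and reloading.
; Damage triggers a camera shake, while fire and reload events play montages on the Arms mesh, with reload guarded by gun state before calling the parent.
; Equipping a gun makes its mesh owner-only and shadowless.
; Crouching offsets FakeBody based on network role, with a debug print and a TODO marking it broken.
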(event `OnTakeAnyDamage Event` :!signature `self.OnTakeAnyDamage`
  (params (DamagedActor :type "Actor Object Reference") (Damage :type "Float (double-precision)") (DamageType :type "DamageType Object Reference") (InstigatedBy :type "Controller Object Reference") (DamageCauser :type "Actor Object Reference"))
  ;[1 1 1] Bind Damage Event to Cam Shake
  (bind _asplayer_controller (cast `PlayerController` (`self.GetController`)))
  (`PlayerCameraManager.PlayCameraShake` :`self` (`PlayerController.PlayerCameraManager` _asplayer_controller) :`ShakeClass` "/Game/Blueprints/BP_CamShake.BP_CamShake_C"))

(event `self.OnGunSet`
  (bind _returnvalue (`self.GetComponentByClass` (`self.GetGun`) "/Script/Engine.SkeletalMeshComponent"))
  ;[1 1 1] Hide the Gun Mesh
  (`PrimitiveComponent.SetOnlyOwnerSee` _returnvalue true)
  (`PrimitiveComponent.SetCastShadow` _returnvalue false))

(event `self.ReceiveBeginPlay`
  ;[1 1 1] Bind Damage Event to Cam Shake
  (add `self.OnTakeAnyDamage` (delegate `OnTakeAnyDamage Event`)))

(event `self.K2_OnStartCrouch`
  (params (HalfHeightAdjust :type "Float (single-precision)") (ScaledHalfHeightAdjust :type "Float (single-precision)"))
  ;[1 1 1] Crouch Adjust (TODO THIS IS BROKEN)
  (if (or (`|EnumEquality` (`self.GetLocalRole`) "ROLE_SimulatedProxy") (`|EnumEquality` (`self.GetRemoteRole`) "ROLE_AutonomousProxy"))
    (`self.CrouchAdjust` ScaledHalfHeightAdjust)))

(event `self.K2_OnEndCrouch`
  (params (HalfHeightAdjust :type "Float (single-precision)") (ScaledHalfHeightAdjust :type "Float (single-precision)"))
  ;[1 1 1] Crouch Adjust (TODO THIS IS BROKEN)
  (if (or (`|EnumEquality` (`self.GetLocalRole`) "ROLE_SimulatedProxy") (`|EnumEquality` (`self.GetRemoteRole`) "ROLE_AutonomousProxy"))
    (`self.CrouchAdjust` (* ScaledHalfHeightAdjust -1.0))))

(event `self.OnFired`
  ;[1 1 1] Play Firing Montage on Arms
  (`AnimInstance.Montage_Play` (`SkeletalMeshComponent.GetAnimInstance` (`self.Arms`)) "/Game/Assets/Arms/Animations/FirstPersonFire_Montage.FirstPersonFire_Montage" 1.0 "MontageLength" 0.0 true))

(event `self.BeginReload`
  (params (Length :type "Float (single-precision)"))
  (bind _returnvalue (`self.GetGun`))
  ;[1 1 1] Play Reload Montage on Arms
  (if (`KismetSystemLibrary.IsValid` _returnvalue)
    (if (and (not (`self.IsReloading`)) (not (`GunBase.FullyLoaded` _returnvalue)))
      (`GameplayStatics.PlaySoundAtLocation` "/Game/Sounds/Reload_Cue.Reload_Cue" (`self.K2_GetActorLocation` _returnvalue) (struct) 1.0 1.0 0.0 null null null)
      (bind _returnvalue_2 (`AnimInstance.Montage_Play` (`SkeletalMeshComponent.GetAnimInstance` (`self.Arms`)) "/Game/Assets/Arms/Animations/FirstPersonReload_Montage.FirstPersonReload_Montage" 1.0 "MontageLength" 0.0 true))
      (`parent.BeginReload` _returnvalue_2))))

(fn `CrouchAdjust`
  (params (CrouchDelta :type "Float (double-precision)"))
  (`SceneComponent.K2_AddRelativeLocation` (`self.FakeBody`) (`KismetMathLibrary.MakeVector` 0.0 0.0 CrouchDelta) false false)
  (`KismetSystemLibrary.PrintString` (`KismetStringLibrary.Conv_DoubleToString` CrouchDelta)))

(fn `OnRep_NewEventDispatcher_0`)

(fn `UserConstructionScript`)